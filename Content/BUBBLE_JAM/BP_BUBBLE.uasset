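; Fire, ice or gum bubble projectile that traps enemies until the player pops it.
; Construction sets speed and scale; BeginPlay sets material, homing target and a catch limit from bar spent.
; Hits and overlaps switch on gameplay tags: enemies attach up to the limit, anchors zero max speed.
; Player contact after charging kills captives, adds killstreak and pops it, granting an elemental trail for fire/ice or refilling the gum bar.
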(event OnComponentBeginOverlap(Sphere1)
  (params (OverlappedComponent :type Primitive%20Component%20Object%20Reference) (OtherActor :type Actor%20Object%20Reference) (OtherComp :type Primitive%20Component%20Object%20Reference) (OtherBodyIndex :type Integer) (bFromSweep :type Boolean) (SweepResult :type Hit%20Result%20Structure%20%28by%20ref%29))
  (bind _ammotype (Variables|Default|GetAmmoType))
  (Variables|Default|SetHitActor OtherActor)
  (bind _tagcontainer (Class|BPIBubbleInterface|GetGameplayTags(Message) (Variables|Default|GetHitActor)))
  (for _array_element (GameplayTags|BreakGameplayTagContainer _tagcontainer)
    (|SwitchGameplayTag _array_element
      (:Player
        (if (not (Variables|Default|GetIsBeingCharged))
          (Utilities|FlowControl|Delay 0.2)
          (bind _foundwidgets (Widget|GetAllWidgetsOfClass "/Game/BUBBLE_JAM/WBP_BubbleUI.WBP_BubbleUI_C" true))
          (switch Utilities|FlowControl|Switch|SwitchonPickups_enum _ammotype
            (:NewEnumerator1
              (Class|BPIBubbleInterface|PlayerElementalTrail(Message) (Game|GetPlayerCharacter 0) _ammotype :!label _label)
              (Class|BPIBubbleInterface|PlayerElementalTrail(Message) (Game|GetPlayerController 0) _ammotype))
            (:NewEnumerator2
              (goto _label))
            (:NewEnumerator3
              (Default|RefillBar (Utilities|Array|Get(acopy) _foundwidgets) (Variables|Default|GetBar%25Used) "NewEnumerator3")))
          (for _array_element_2 (Variables|Default|GetCapturedActors)
            (Class|BPIBubbleInterface|EnemyDeath(Message) _array_element_2)
            (Class|BPIBubbleInterface|ChangeKillstreak(Message) (Game|GetPlayerController 0) true false))
          (Audio|PlaySound2D "/Game/BUBBLE_JAM/SFX/bubble_pop.bubble_pop" 1.0 1.0 0.0 0 0)
          (Actor|DestroyActor)))
      (:Enemy
        (if (and (> (Variables|Default|GetCatchLimit) 0) (not (Utilities|Array|ContainsItem (Variables|Default|GetCapturedActors) (Variables|Default|GetHitActor))))
          (Utilities|FlowControl|DoOnce false :!label _label_2
            (:Completed
              (Transformation|AttachActorToActor (Variables|Default|GetHitActor) self (Utilities|Array|Get(acopy) (Transformation|GetAllSocketNames (Variables|Default|GetSphere))) "SnapToTarget" "KeepRelative" "SnapToTarget" false)
              (Class|BPIBubbleInterface|STOP(Message) (Variables|Default|GetHitActor))
              (Utilities|Array|AddUnique (Variables|Default|GetCapturedActors) (Variables|Default|GetHitActor))
              (Math|Integer|DecrementInt (Variables|Default|GetCatchLimit)
                (:%20%20
                  (goto _label_2 Reset)))))))
      (:BubbleAnchor
        (Variables|/Script/Engine.ProjectileMovementComponent|SetMaxSpeed (Variables|Default|GetProjectileMovement) 0.0)))))

(event EventSTOP
  (Variables|/Script/Engine.ProjectileMovementComponent|SetMaxSpeed (Variables|Default|GetProjectileMovement) 0.0)
  (Development|PrintString "BUBBLESTOP")
  (Development|PrintString (Utilities|String|ToString(Float) (Class|MovementComponent|GetMaxSpeed (Variables|Default|GetProjectileMovement))))
  (Game|Components|ProjectileMovement|StopSimulating (Variables|Default|GetProjectileMovement) (Collision|MakeHitResult false false 0.0 0.0 "0, 0, 0" "0, 0, 0" "0,0,1" "0,0,1" 0 0)))

(event EventBeginPlay
  (bind _sphere (Variables|Default|GetSphere))
  (Variables|/Script/Engine.ProjectileMovementComponent|SetHomingTargetComponent (Variables|Default|GetProjectileMovement) (Variables|Default|GetHoming%20Target%20Component))
  (Utilities|FlowControl|Delay 0.05)
  (Variables|Default|SetIsBeingCharged false)
  (Variables|Default|SetCatchLimit (Math|Float|Truncate (/ (Variables|Default|GetBar%25Used) 0.11)))
  (switch Utilities|FlowControl|Switch|SwitchonPickups_enum (Variables|Default|GetAmmoType)
    (:NewEnumerator1
      (Rendering|Material|SetMaterial _sphere 0 "/Game/BUBBLE_JAM/MI_Pyramid_03.MI_Pyramid_03"))
    (:NewEnumerator2
      (Rendering|Material|SetMaterial _sphere 0 "/Game/BUBBLE_JAM/MI_Pyramid_05.MI_Pyramid_05"))
    (:NewEnumerator3
      (Rendering|Material|SetMaterial _sphere 0 "/Engine/VREditor/BasicMeshes/MI_Pyramid_01.MI_Pyramid_01"))))

(event Collision|EventHit
  (params (MyComp :type Primitive%20Component%20Object%20Reference) (Other :type Actor%20Object%20Reference) (OtherComp :type Primitive%20Component%20Object%20Reference) (bSelfMoved :type Boolean) (HitLocation :type Vector :default "0, 0, 0") (HitNormal :type Vector :default "0, 0, 0") (NormalImpulse :type Vector :default "0, 0, 0") (Hit :type Hit%20Result%20Structure%20%28by%20ref%29))
  (bind _ammotype (Variables|Default|GetAmmoType))
  (Variables|Default|SetHitActor Other)
  (bind _tagcontainer (Class|BPIBubbleInterface|GetGameplayTags(Message) (Variables|Default|GetHitActor)))
  (for _array_element (GameplayTags|BreakGameplayTagContainer _tagcontainer)
    (|SwitchGameplayTag _array_element
      (:Player
        (if (not (Variables|Default|GetIsBeingCharged))
          (Utilities|FlowControl|Delay 0.2)
          (bind _foundwidgets (Widget|GetAllWidgetsOfClass "/Game/BUBBLE_JAM/WBP_BubbleUI.WBP_BubbleUI_C" true))
          (switch Utilities|FlowControl|Switch|SwitchonPickups_enum _ammotype
            (:NewEnumerator1
              (Class|BPIBubbleInterface|PlayerElementalTrail(Message) (Game|GetPlayerCharacter 0) _ammotype :!label _label)
              (Class|BPIBubbleInterface|PlayerElementalTrail(Message) (Game|GetPlayerController 0) _ammotype))
            (:NewEnumerator2
              (goto _label))
            (:NewEnumerator3
              (Default|RefillBar (Utilities|Array|Get(acopy) _foundwidgets) (Variables|Default|GetBar%25Used) "NewEnumerator3")))
          (for _array_element_2 (Variables|Default|GetCapturedActors)
            (Class|BPIBubbleInterface|EnemyDeath(Message) _array_element_2)
            (Class|BPIBubbleInterface|ChangeKillstreak(Message) (Game|GetPlayerController 0) true false))
          (Audio|PlaySound2D "/Game/BUBBLE_JAM/SFX/bubble_pop.bubble_pop" 1.0 1.0 0.0 0 0)
          (Actor|DestroyActor)))
      (:Enemy
        (if (and (> (Variables|Default|GetCatchLimit) 0) (not (Utilities|Array|ContainsItem (Variables|Default|GetCapturedActors) (Variables|Default|GetHitActor))))
          (Utilities|FlowControl|DoOnce false :!label _label_2
            (:Completed
              (Transformation|AttachActorToActor (Variables|Default|GetHitActor) self (Utilities|Array|Get(acopy) (Transformation|GetAllSocketNames (Variables|Default|GetSphere))) "SnapToTarget" "KeepRelative" "SnapToTarget" false)
              (Class|BPIBubbleInterface|STOP(Message) (Variables|Default|GetHitActor))
              (Utilities|Array|AddUnique (Variables|Default|GetCapturedActors) (Variables|Default|GetHitActor))
              (Math|Integer|DecrementInt (Variables|Default|GetCatchLimit)
                (:%20%20
                  (goto _label_2 Reset)))))))
      (:BubbleAnchor
        (Variables|/Script/Engine.ProjectileMovementComponent|SetMaxSpeed (Variables|Default|GetProjectileMovement) 0.0)))))

(fn ConstructionScript
  (bind _projectilemovement (Variables|Default|GetProjectileMovement))
  (bind _sphere (Variables|Default|GetSphere))
  (bind _output_get (Variables|/Script/Engine.ProjectileMovementComponent|SetMaxSpeed _projectilemovement (+ (Variables|Default|GetSPEED_Inherited) (Variables|Default|GetSPEED_Self))))
  (Variables|/Script/Engine.ProjectileMovementComponent|SetInitialSpeed _projectilemovement _output_get)
  (Transformation|SetActorScale3D (Math|Conversions|ToVector(Float) (Variables|Default|GetScale)))
  (switch Utilities|FlowControl|Switch|SwitchonPickups_enum (Variables|Default|GetAmmoType)
    (:NewEnumerator1
      (Rendering|Material|SetMaterial _sphere 0 0))
    (:NewEnumerator2
      (Rendering|Material|SetMaterial _sphere 0 0))
    (:NewEnumerator3
      (Rendering|Material|SetMaterial _sphere 0 "/Engine/VREditor/BasicMeshes/MI_Pyramid_01.MI_Pyramid_01"))))

(fn GetGameplayTags
  (return (Variables|Default|GetGameplayTags)))

(fn GetSpeedUpMult
  (return (* (Variables|Default|GetScale) 2.0)))