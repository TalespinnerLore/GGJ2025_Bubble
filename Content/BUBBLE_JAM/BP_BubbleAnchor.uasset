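; BP_BubbleAnchor is a short-lived anchor actor that stops a bubble on contact and is then used up.
; It sets a five-second lifespan on BeginPlay.
; On capsule overlap, it reads the other actor's gameplay tags through a message call and, for a BUBBLE tag, sends STOP and destroys itself.
; A capsule hit by a BP_BUBBLE also destroys it after a brief delay, without sending STOP.
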(event OnComponentBeginOverlap(Capsule)
  (params (OverlappedComponent :type Primitive%20Component%20Object%20Reference) (OtherActor :type Actor%20Object%20Reference) (OtherComp :type Primitive%20Component%20Object%20Reference) (OtherBodyIndex :type Integer) (bFromSweep :type Boolean) (SweepResult :type Hit%20Result%20Structure%20%28by%20ref%29))
  (bind _output_get (Variables|Default|SetOverlapActor OtherActor))
  (bind _tagcontainer (Class|BPIBubbleInterface|GetGameplayTags(Message) _output_get))
  (for _array_element (GameplayTags|BreakGameplayTagContainer _tagcontainer)
    (|SwitchGameplayTag _array_element
      (:BUBBLE
        (Class|BPIBubbleInterface|STOP(Message) (Variables|Default|GetOverlapActor))
        (Actor|DestroyActor)))))

(event OnComponentHit(Capsule)
  (params (HitComponent :type Primitive%20Component%20Object%20Reference) (OtherActor :type Actor%20Object%20Reference) (OtherComp :type Primitive%20Component%20Object%20Reference) (NormalImpulse :type Vector :default "0, 0, 0") (Hit :type Hit%20Result%20Structure%20%28by%20ref%29))
  (Utilities|FlowControl|Delay 0.1)
  (if (== (Utilities|GetClass OtherActor) "/Game/BUBBLE_JAM/BP_BUBBLE.BP_BUBBLE_C")
    (Actor|DestroyActor)))

(event EventBeginPlay
  (Actor|SetLifeSpan 5.0))

(event Collision|EventActorBeginOverlap
  (params (OtherActor :type Actor%20Object%20Reference)))

(event EventTick
  (params (DeltaSeconds :type Float%20%28single-precision%29)))

(fn ConstructionScript)