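; Enemy pawn Blueprint for the BUBBLE_JAM game that explodes and destroys itself shortly after overlapping the player character.
; EnemyDeath destroys it and sometimes spawns a BP_Pickup at a fixed height, with a weighted random type.
; A STOP event halts controller movement, while getter functions supply its gameplay tags and a constant speed-up multiplier.
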(event EventBeginPlay)

(event Collision|EventActorBeginOverlap
  (params (OtherActor :type Actor%20Object%20Reference))
  (Utilities|FlowControl|Delay 0.05)
  (if (== OtherActor (Game|GetPlayerCharacter 0))
    (Effects|SpawnEmitteratLocation "/Game/StarterContent/Particles/P_Explosion.P_Explosion" (Transformation|GetActorLocation))
    (Actor|DestroyActor)))

(event EventSTOP
  (AI|Navigation|StopMovement (Pawn|GetController)))

(event EventEnemyDeath
  (bind _returnvalue (Transformation|GetActorLocation))
  (if (Math|Random|RandomBoolwithWeight 0.45)
    (bind _output_get (Variables|Default|SetDropLocation (Math|Vector|MakeVector (.x _returnvalue) (.y _returnvalue) 5e+01)))
    (Game|SpawnActorfromClass "/Game/BUBBLE_JAM/BP_Pickup.BP_Pickup_C" (Math|Conversions|ToTransform(Vector) _output_get) "Undefined" "MultiplyWithRoot" 0 (select (Math|Random|RandomBoolwithWeight 0.6) "NewEnumerator0" (select (Math|Random|RandomBool) "NewEnumerator2" "NewEnumerator1")) 0)
    (Actor|DestroyActor)
    (else
      (Actor|DestroyActor))))

(fn ConstructionScript)

(fn GetGameplayTags
  (return (Variables|Default|GetGameplayTags)))

(fn GetSpeedUpMult
  (return 1.5))