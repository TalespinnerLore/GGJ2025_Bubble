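; BP_EffectTrail is a short-lived effect actor that acts as either a fire or ice trail, selected by its Type.
; On BeginPlay it attaches the matching particle effect to its Box and sets a type-specific lifespan.
; When another actor overlaps it, the fire type sends that actor EnemyScreenExplodeMessage, while the ice type has no overlap effect.
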(event EventBeginPlay
  (bind _box (Variables|Default|GetBox))
  (switch Utilities|FlowControl|Switch|SwitchonPickups_enum (Variables|Default|GetType#)
    (:NewEnumerator1
      (Effects|SpawnEmitterAttached "/Game/StarterContent/Particles/P_Fire.P_Fire" _box "None" "0, 0, 0" "0, 0, 0" "1.000000,1.000000,1.000000" "SnapToTarget" false)
      (Actor|SetLifeSpan 3.0))
    (:NewEnumerator2
      (Niagara|SpawnSystemAttached "/Game/StarterContent/Particles/IceParticels.IceParticels" _box "None" "0, 0, 0" "0, 0, 0" "SnapToTarget" false)
      (Actor|SetLifeSpan 2.0))))

(event Collision|EventActorBeginOverlap
  (params (OtherActor :type Actor%20Object%20Reference))
  (switch Utilities|FlowControl|Switch|SwitchonPickups_enum (Variables|Default|GetType#)
    (:NewEnumerator1
      (Class|BPIBubbleInterface|EnemyScreenExplode(Message) OtherActor))))

(event EventTick
  (params (DeltaSeconds :type Float%20%28single-precision%29)))

(fn ConstructionScript)