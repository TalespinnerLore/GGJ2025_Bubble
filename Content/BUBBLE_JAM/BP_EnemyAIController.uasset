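; Enemy AI controller that sends its pawn toward the player's top-down character.
; Shortly after BeginPlay it looks up the BP_TopDownCharacter, issues a single MoveToActor toward it and prints whether that reference is valid.
; A STOP event routes to StopPossessing, which unpossesses the pawn.
; GetGameplayTags and GetSpeedUpMult are stubs returning empty or zero, and Tick and the construction script do nothing.
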(event Custom|StopPossessing
  (Pawn|UnPossess))

(event EventBeginPlay
  (Utilities|FlowControl|Delay 0.2)
  (bind _returnvalue (Actor|GetActorOfClass "/Game/BUBBLE_JAM/BP_TopDownCharacter.BP_TopDownCharacter_C"))
  (AI|Navigation|MovetoActor _returnvalue -1.0 true true true 0)
  (Development|PrintString (Utilities|String|ToString(Boolean) (Utilities|IsValid _returnvalue))))

(event EventTick
  (params (DeltaSeconds :type Float%20%28single-precision%29)))

(event EventSTOP
  (CallFunction|StopPossessing))

(fn ConstructionScript)

(fn GetGameplayTags
  (return ""))

(fn GetSpeedUpMult
  (return 0.0))