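; Enemy spawner actor that sends in waves of BP_ENEMY that grow over time.
; On BeginPlay it spawns a wave at once, then repeats on a looping 20-second timer.
; Each enemy appears at a random distance along the actor's spline, adjusted for collisions but always spawned.
; After every wave the Enemy count rises by two, so waves escalate without limit.
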(event Custom|SpawnWave
  (bind _spline (Variables|Default|GetSpline))
  (for _index (range 0 (Variables|Default|GetEnemy#))
    (Game|SpawnActorfromClass "/Game/BUBBLE_JAM/BP_ENEMY.BP_ENEMY_C" (Spline|GetTransformatDistanceAlongSpline _spline (Math|Random|RandomFloatinRange 0.0 (Spline|GetSplineLength _spline)) "World" true) "AdjustIfPossibleButAlwaysSpawn" "MultiplyWithRoot" 0 0))
  (Variables|Default|SetEnemy# (+ (Variables|Default|GetEnemy#) 2)))

(event EventBeginPlay
  (Utilities|Time|SetTimerbyEvent (delegate Custom|SpawnWave) 2e+01 true)
  (CallFunction|SpawnWave))

(event Collision|EventActorBeginOverlap
  (params (OtherActor :type Actor%20Object%20Reference)))

(event EventTick
  (params (DeltaSeconds :type Float%20%28single-precision%29)))

(fn ConstructionScript)