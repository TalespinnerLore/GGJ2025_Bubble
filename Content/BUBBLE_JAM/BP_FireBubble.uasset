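; BP_FireBubble is a charged homing projectile that captures enemies and pops when it touches the player.
; Speed and scale are set at construction, and capture capacity derives from BarUsed.
; Hit and overlap share a gameplay-tag switch: enemies get attached and stopped up to the limit, and Bubble Anchors zero max speed.
; Player contact after charging sends a fire-trail message, kills captured enemies after a short delay and destroys the bubble.
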(event OnComponentBeginOverlap(Sphere1)
  (params (OverlappedComponent :type Primitive%20Component%20Object%20Reference) (OtherActor :type Actor%20Object%20Reference) (OtherComp :type Primitive%20Component%20Object%20Reference) (OtherBodyIndex :type Integer) (bFromSweep :type Boolean) (SweepResult :type Hit%20Result%20Structure%20%28by%20ref%29))
  (Variables|Default|SetHitActor OtherActor)
  (bind _tagcontainer (Class|BPIBubbleInterface|GetGameplayTags(Message) (Variables|Default|GetHitActor)))
  (for _array_element (GameplayTags|BreakGameplayTagContainer _tagcontainer)
    (|SwitchGameplayTag _array_element
      (:Player
        (if (not (Variables|Default|GetIsBeingCharged))
          (Class|BPIBubbleInterface|PlayerFireTrail(Message) (Game|GetPlayerCharacter 0))
          (Utilities|FlowControl|Delay 0.2)
          (for _array_element_2 (Variables|Default|GetCapturedActors)
            (Class|BPIBubbleInterface|EnemyDeath(Message) _array_element_2))
          ;[1 0 0] SFX NEEDED
          (Audio|PlaySound2D 0 1.0 1.0 0.0 0 0)
          (Actor|DestroyActor)))
      (:Enemy
        (if (and (> (Variables|Default|GetCatchLimit) 0) (not (Utilities|Array|ContainsItem (Variables|Default|GetCapturedActors) (Variables|Default|GetHitActor))))
          (Utilities|FlowControl|DoOnce false :!label _label
            (:Completed
              (Transformation|AttachActorToActor (Variables|Default|GetHitActor) self (Utilities|Array|Get(acopy) (Transformation|GetAllSocketNames (Variables|Default|GetSphere))) "SnapToTarget" "KeepRelative" "SnapToTarget" false)
              (Class|BPIBubbleInterface|STOP(Message) (Variables|Default|GetHitActor))
              (Utilities|Array|AddUnique (Variables|Default|GetCapturedActors) (Variables|Default|GetHitActor))
              (Math|Integer|DecrementInt (Variables|Default|GetCatchLimit)
                (:%20%20
                  (goto _label Reset)))))))
      (:BubbleAnchor
        (Variables|/Script/Engine.ProjectileMovementComponent|SetMaxSpeed (Variables|Default|GetProjectileMovement) 0.0)))))

(event EventSTOP
  (Variables|/Script/Engine.ProjectileMovementComponent|SetMaxSpeed (Variables|Default|GetProjectileMovement) 0.0)
  (Development|PrintString "BUBBLESTOP")
  (Development|PrintString (Utilities|String|ToString(Float) (Class|MovementComponent|GetMaxSpeed (Variables|Default|GetProjectileMovement))))
  (Game|Components|ProjectileMovement|StopSimulating (Variables|Default|GetProjectileMovement) (Collision|MakeHitResult false false 0.0 0.0 "0, 0, 0" "0, 0, 0" "0,0,1" "0,0,1" 0 0)))

(event EventBeginPlay
  (Variables|/Script/Engine.ProjectileMovementComponent|SetHomingTargetComponent (Variables|Default|GetProjectileMovement) (Variables|Default|GetHoming%20Target%20Component))
  (Utilities|FlowControl|Delay 0.05)
  (Variables|Default|SetIsBeingCharged false)
  (Variables|Default|SetCatchLimit (Math|Float|Truncate (/ (Variables|Default|GetBar%25Used) 0.11))))

(event Collision|EventHit
  (params (MyComp :type Primitive%20Component%20Object%20Reference) (Other :type Actor%20Object%20Reference) (OtherComp :type Primitive%20Component%20Object%20Reference) (bSelfMoved :type Boolean) (HitLocation :type Vector :default "0, 0, 0") (HitNormal :type Vector :default "0, 0, 0") (NormalImpulse :type Vector :default "0, 0, 0") (Hit :type Hit%20Result%20Structure%20%28by%20ref%29))
  (Variables|Default|SetHitActor Other)
  (bind _tagcontainer (Class|BPIBubbleInterface|GetGameplayTags(Message) (Variables|Default|GetHitActor)))
  (for _array_element (GameplayTags|BreakGameplayTagContainer _tagcontainer)
    (|SwitchGameplayTag _array_element
      (:Player
        (if (not (Variables|Default|GetIsBeingCharged))
          (Class|BPIBubbleInterface|PlayerFireTrail(Message) (Game|GetPlayerCharacter 0))
          (Utilities|FlowControl|Delay 0.2)
          (for _array_element_2 (Variables|Default|GetCapturedActors)
            (Class|BPIBubbleInterface|EnemyDeath(Message) _array_element_2))
          ;[1 0 0] SFX NEEDED
          (Audio|PlaySound2D 0 1.0 1.0 0.0 0 0)
          (Actor|DestroyActor)))
      (:Enemy
        (if (and (> (Variables|Default|GetCatchLimit) 0) (not (Utilities|Array|ContainsItem (Variables|Default|GetCapturedActors) (Variables|Default|GetHitActor))))
          (Utilities|FlowControl|DoOnce false :!label _label
            (:Completed
              (Transformation|AttachActorToActor (Variables|Default|GetHitActor) self (Utilities|Array|Get(acopy) (Transformation|GetAllSocketNames (Variables|Default|GetSphere))) "SnapToTarget" "KeepRelative" "SnapToTarget" false)
              (Class|BPIBubbleInterface|STOP(Message) (Variables|Default|GetHitActor))
              (Utilities|Array|AddUnique (Variables|Default|GetCapturedActors) (Variables|Default|GetHitActor))
              (Math|Integer|DecrementInt (Variables|Default|GetCatchLimit)
                (:%20%20
                  (goto _label Reset)))))))
      (:BubbleAnchor
        (Variables|/Script/Engine.ProjectileMovementComponent|SetMaxSpeed (Variables|Default|GetProjectileMovement) 0.0)))))

(fn ConstructionScript
  (bind _projectilemovement (Variables|Default|GetProjectileMovement))
  (bind _output_get (Variables|/Script/Engine.ProjectileMovementComponent|SetMaxSpeed _projectilemovement (+ (Variables|Default|GetSPEED_Inherited) (Variables|Default|GetSPEED_Self))))
  (Variables|/Script/Engine.ProjectileMovementComponent|SetInitialSpeed _projectilemovement _output_get)
  (Transformation|SetActorScale3D (Math|Conversions|ToVector(Float) (Variables|Default|GetScale)))
  (Development|PrintString (Utilities|String|ToString(Float) (Class|MovementComponent|GetMaxSpeed (Variables|Default|GetProjectileMovement)))))

(fn GetGameplayTags
  (return (Variables|Default|GetGameplayTags)))

(fn GetSpeedUpMult
  (return (* (Variables|Default|GetScale) 2.0)))