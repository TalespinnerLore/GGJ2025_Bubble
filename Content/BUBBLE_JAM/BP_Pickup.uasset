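; BP_Pickup is a collectible that grants the player HP or charges a FIRE, ICE or GUM element bar.
; On BeginPlay its Type sets the Sphere's material, with FIRE and ICE sharing the same one.
; Actor overlap and Sphere1 overlap share one path: for an exact BP_TopDownCharacter class match, it sends the matching message to player character 0 and destroys itself.
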(event OnComponentBeginOverlap(Sphere1)
  (params (OverlappedComponent :type Primitive%20Component%20Object%20Reference) (OtherActor :type Actor%20Object%20Reference) (OtherComp :type Primitive%20Component%20Object%20Reference) (OtherBodyIndex :type Integer) (bFromSweep :type Boolean) (SweepResult :type Hit%20Result%20Structure%20%28by%20ref%29))
  (bind _returnvalue (Game|GetPlayerCharacter 0))
  (if (== (Utilities|GetClass OtherActor) "/Game/BUBBLE_JAM/BP_TopDownCharacter.BP_TopDownCharacter_C")
    (switch Utilities|FlowControl|Switch|SwitchonPickups_enum (Variables|Default|GetType)
      (:NewEnumerator0
        (Class|BPIBubbleInterface|AddHP(Message) _returnvalue))
      (:NewEnumerator1
        (Class|BPIBubbleInterface|ChargeElementBar(Message) _returnvalue "NewEnumerator1"))
      (:NewEnumerator2
        (Class|BPIBubbleInterface|ChargeElementBar(Message) _returnvalue "NewEnumerator2"))
      (:NewEnumerator3
        (Class|BPIBubbleInterface|ChargeElementBar(Message) _returnvalue "NewEnumerator3")))
    (Actor|DestroyActor)))

(event EventBeginPlay
  (switch Utilities|FlowControl|Switch|SwitchonPickups_enum (Variables|Default|GetType)
    (:NewEnumerator0
      (Rendering|Material|SetMaterial (Variables|Default|GetSphere) 0 "/Engine/MapTemplates/Materials/BasicAsset03.BasicAsset03"))
    (:NewEnumerator1
      (Rendering|Material|SetMaterial (Variables|Default|GetSphere) 0 "/Engine/VREditor/BasicMeshes/MI_Pyramid_04.MI_Pyramid_04"))
    (:NewEnumerator2
      (Rendering|Material|SetMaterial (Variables|Default|GetSphere) 0 "/Engine/VREditor/BasicMeshes/MI_Pyramid_04.MI_Pyramid_04"))
    (:NewEnumerator3
      (Rendering|Material|SetMaterial (Variables|Default|GetSphere) 0 "/Engine/VREditor/BasicMeshes/MI_Pyramid_01.MI_Pyramid_01"))))

(event Collision|EventActorBeginOverlap
  (params (OtherActor :type Actor%20Object%20Reference))
  (bind _returnvalue (Game|GetPlayerCharacter 0))
  (if (== (Utilities|GetClass OtherActor) "/Game/BUBBLE_JAM/BP_TopDownCharacter.BP_TopDownCharacter_C")
    (switch Utilities|FlowControl|Switch|SwitchonPickups_enum (Variables|Default|GetType)
      (:NewEnumerator0
        (Class|BPIBubbleInterface|AddHP(Message) _returnvalue))
      (:NewEnumerator1
        (Class|BPIBubbleInterface|ChargeElementBar(Message) _returnvalue "NewEnumerator1"))
      (:NewEnumerator2
        (Class|BPIBubbleInterface|ChargeElementBar(Message) _returnvalue "NewEnumerator2"))
      (:NewEnumerator3
        (Class|BPIBubbleInterface|ChargeElementBar(Message) _returnvalue "NewEnumerator3")))
    (Actor|DestroyActor)))

(fn ConstructionScript)